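; Police officer enemy character that chases the player and plays an attack animation on reaching them.
; PawnSensing sight sets a seen flag and calls FollowPlayer, which runs AI Move To toward the player and, on success, plays the attack montage followed by a cooldown.
; Tick halts movement until the player is seen; the flag is never cleared afterwards, and each sighting re-arms the attack gate.
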(event OnSeePawn(PawnSensing)
  (params (Pawn :type Pawn%20Object%20Reference))
  (Variables|Default|SetisSeingPlayer true)
  (CallFunction|FollowPlayer))

(event OnHearNoise(PawnSensing)
  (params (Instigator :type Pawn%20Object%20Reference) (Location :type Vector%20%28by%20ref%29 :default "0, 0, 0") (Volume :type Float%20%28single-precision%29)))

(event Custom|FollowPlayer
  (Variables|Default|SetcanAttack true)
  (if (Variables|Default|GetisSeingPlayer)
    (AI|AIMoveTo self "0, 0, 0" (Game|GetPlayerCharacter 0) 9e+01 true
      (:OnSuccess
        (if (Variables|Default|GetcanAttack)
          (Variables|Default|SetcanAttack false)
          (bind _returnvalue (Animation|PlayAnimMontage "/Game/Characters/Police/A_Police_Attack_Montage.A_Police_Attack_Montage" 1.0 "None"))
          (Utilities|FlowControl|Delay (+ _returnvalue (Variables|Default|GetAttackCooldown)))
          (Variables|Default|SetcanAttack true)
          (Development|PrintString "can attack again"))))
    (else
      (Variables|Default|SetisSeingPlayer false))))

(event EventBeginPlay)

(event Collision|EventActorBeginOverlap
  (params (OtherActor :type Actor%20Object%20Reference)))

(event EventTick
  (params (DeltaSeconds :type Float%20%28single-precision%29))
  (if (not (Variables|Default|GetisSeingPlayer))
    (Components|Movement|StopMovementImmediately (Variables|Character|GetCharacterMovement))))

(fn ConstructionScript)